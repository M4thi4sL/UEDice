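; PC_Camera is a player controller that sets up the dice overlay UI and mouse interaction for a dice-throwing scene.
; On BeginPlay it adds WBP_DiceOverlay to the viewport, caches the DiceThrower actor, and switches to Game and UI input with cursor, click and mouse-over events enabled.
; An R debug key clears and respawns the dice through that DiceThrower.
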(event EventBeginPlay
  (bind _returnvalue (UserInterface|CreateWidget "/Game/Widgets/WBP_DiceOverlay.WBP_DiceOverlay_C"))
  (UserInterface|Viewport|AddtoViewport _returnvalue 0)
  (bind _returnvalue_2 (Actor|GetActorOfClass "/Script/Dice.DiceThrower"))
  (Variables|Default|SetDiceThrower _returnvalue_2)
  (Input|SetInputModeGameandUI (Game|GetPlayerController 0) _returnvalue "DoNotLock" false false)
  (Variables|Default|SetbShowMouseCursor true)
  (Variables|Default|SetbEnableMouseOverEvents true)
  (Variables|Default|SetbEnableClickEvents true))

(event Input|KeyboardEvents|DebugKeyR
  (params (Key :type Key%20Structure :default "None") (ActionValue :type Input%20Action%20Value%20Structure))
  (bind _dicethrower (Variables|Default|GetDiceThrower))
  (:Pressed
    (Class|DiceThrower|ClearDice _dicethrower)
    (Class|DiceThrower|SpawnDice _dicethrower)))

(fn ConstructionScript)