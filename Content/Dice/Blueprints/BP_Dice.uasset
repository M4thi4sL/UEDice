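; Dice Blueprint that checks whether the die's orientation matches a known face normal, as a debug validity test.
; BeginPlay blocking-loads the DiceData asset, then compares the mesh's world right vector against each FaceNormals entry per axis within ErrorTolerance, breaking on a match.
; Tick re-enters the same loop every frame, and the result prints as Valid or INVALID without identifying which face matched.
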(event EventBeginPlay
  (bind _dicedata (Variables|Default|GetDiceData))
  (bind _error_tolerance (Variables|Default|GetError%20Tolerance))
  (bind _dicemeshcomponent (Variables|Default|GetDiceMeshComponent))
  (bind _returnvalue (Math|Vector|GetRightVector _dicemeshcomponent))
  (bind (_x _y _z) (Math|Vector|BreakVector _returnvalue))
  (Utilities|LoadAssetBlocking _dicedata)
  (bind _array_element (Utilities|Array|ForEachLoopwithBreak (Variables|/Script/Dice.PDA_Dice|GetFaceNormals (Utilities|ResolveSoftReference _dicedata)) :!label _label)
    (:LoopBody
      (if (Math|Boolean|ANDBoolean (Math|Float|NearlyEqual(Float) (.X (Math|Vector|BreakVector _array_element)) _x _error_tolerance) (Math|Float|NearlyEqual(Float) (.Y (Math|Vector|BreakVector _array_element)) _y _error_tolerance) (Math|Float|NearlyEqual(Float) (.Z (Math|Vector|BreakVector _array_element)) _z _error_tolerance))
        (Variables|Default|SetNewVar (Math|Boolean|ANDBoolean (Math|Float|NearlyEqual(Float) (.X (Math|Vector|BreakVector _array_element)) _x _error_tolerance) (Math|Float|NearlyEqual(Float) (.Y (Math|Vector|BreakVector _array_element)) _y _error_tolerance) (Math|Float|NearlyEqual(Float) (.Z (Math|Vector|BreakVector _array_element)) _z _error_tolerance)))
        (goto _label Break)
        (else
          (Variables|Default|SetNewVar false))))
    (:Completed
      (Development|PrintString (Utilities|String|SelectString "Valid" "INVALID" (Variables|Default|GetNewVar))))))

(event EventTick
  (params (DeltaSeconds :type Float%20%28single-precision%29))
  (bind _error_tolerance (Variables|Default|GetError%20Tolerance))
  (bind _dicemeshcomponent (Variables|Default|GetDiceMeshComponent))
  (bind _returnvalue (Math|Vector|GetRightVector _dicemeshcomponent))
  (bind (_x _y _z) (Math|Vector|BreakVector _returnvalue))
  (bind _array_element (Utilities|Array|ForEachLoopwithBreak (Variables|/Script/Dice.PDA_Dice|GetFaceNormals (Utilities|ResolveSoftReference (Variables|Default|GetDiceData))) :!label _label)
    (:LoopBody
      (if (Math|Boolean|ANDBoolean (Math|Float|NearlyEqual(Float) (.X (Math|Vector|BreakVector _array_element)) _x _error_tolerance) (Math|Float|NearlyEqual(Float) (.Y (Math|Vector|BreakVector _array_element)) _y _error_tolerance) (Math|Float|NearlyEqual(Float) (.Z (Math|Vector|BreakVector _array_element)) _z _error_tolerance))
        (Variables|Default|SetNewVar (Math|Boolean|ANDBoolean (Math|Float|NearlyEqual(Float) (.X (Math|Vector|BreakVector _array_element)) _x _error_tolerance) (Math|Float|NearlyEqual(Float) (.Y (Math|Vector|BreakVector _array_element)) _y _error_tolerance) (Math|Float|NearlyEqual(Float) (.Z (Math|Vector|BreakVector _array_element)) _z _error_tolerance)))
        (goto _label Break)
        (else
          (Variables|Default|SetNewVar false))))
    (:Completed
      (Development|PrintString (Utilities|String|SelectString "Valid" "INVALID" (Variables|Default|GetNewVar))))))

(fn ConstructionScript)